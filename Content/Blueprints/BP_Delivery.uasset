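; BP_Delivery is a delivery point that takes a package from the cow player character in exchange for money.
; Tick shows the player's distance in meters on a waypoint widget and, when the player is slow, checks the last actor to overlap the Box.
; If that cow carries packages and the point is available, it updates packages and money, hides itself and re-enables game mode spawning.
; The money HUD update is disconnected.
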(event OnComponentBeginOverlap(Box)
  (params (OverlappedComponent :type Primitive%20Component%20Object%20Reference) (OtherActor :type Actor%20Object%20Reference) (OtherComp :type Primitive%20Component%20Object%20Reference) (OtherBodyIndex :type Integer) (bFromSweep :type Boolean) (SweepResult :type Hit%20Result%20Structure%20%28by%20ref%29))
  (Development|PrintString "Ha entrado"))

(event OnComponentEndOverlap(Box)
  (params (OverlappedComponent :type Primitive%20Component%20Object%20Reference) (OtherActor :type Actor%20Object%20Reference) (OtherComp :type Primitive%20Component%20Object%20Reference) (OtherBodyIndex :type Integer))
  (Variables|Default|Setdentro? false))

(event EventBeginPlay
  (bind _aswd_waypoint_delivery (Utilities|Casting|CastToWD_Waypoint_Delivery (UserInterface|GetWidget (Variables|Default|GetWaypointWidget))))
  (Variables|Default|SetDistance (Variables|/Game/UI/WD_Waypoint_Delivery.WD_Waypoint_Delivery_C|GetDistance _aswd_waypoint_delivery)))

(event Collision|EventActorBeginOverlap
  (params (OtherActor :type Actor%20Object%20Reference)))

(event EventTick
  (params (DeltaSeconds :type Float%20%28single-precision%29))
  (Rendering|Components|TextRender|SetText (Variables|Default|GetDistance) (Utilities|Text|ToText(String) (Utilities|String|Append (Utilities|String|ToString(Integer) (Math|Float|Truncate (/ (Math|Vector|Distance(Vector) (Transformation|GetActorLocation) (Transformation|GetActorLocation (Game|Player|GetPlayerPawn 0))) 1e+02))) " m")))
  (bind _asbp_third_person_character_cow (Utilities|Casting|CastToBP_ThirdPersonCharacterCow (Game|GetPlayerCharacter 0)))
  (if (<= (Math|Vector|VectorLength (Transformation|GetVelocity _asbp_third_person_character_cow)) 1e+02)
    (Variables|Default|Setdentro? true)
    (bind _asbp_third_person_character_cow_2 (Utilities|Casting|CastToBP_ThirdPersonCharacterCow (stale OnComponentBeginOverlap(Box) OtherActor)))
    (if (Variables|Default|Getdentro?)
      (if (> (Variables|/Game/ThirdPerson/Blueprints/BP_ThirdPersonCharacterCow.BP_ThirdPersonCharacterCow_C|GetNumberOfPackages _asbp_third_person_character_cow_2) 0)
        (if (Variables|Default|GetDisponible?)
          (bind _result (Math|Integer|DecrementInt (Variables|/Game/ThirdPerson/Blueprints/BP_ThirdPersonCharacterCow.BP_ThirdPersonCharacterCow_C|GetNumberOfPackages _asbp_third_person_character_cow_2))
            (:%20%20
              (bind _output_get (Variables|/Game/ThirdPerson/Blueprints/BP_ThirdPersonCharacterCow.BP_ThirdPersonCharacterCow_C|SetNumberOfPackages _asbp_third_person_character_cow_2 _result))
              (Default|SetTxtPackages (Variables|/Game/ThirdPerson/Blueprints/BP_ThirdPersonCharacterCow.BP_ThirdPersonCharacterCow_C|GetHUD _asbp_third_person_character_cow_2) _output_get)
              (bind _output_get_2 (Variables|/Game/ThirdPerson/Blueprints/BP_ThirdPersonCharacterCow.BP_ThirdPersonCharacterCow_C|SetMoney _asbp_third_person_character_cow_2 (+ (Variables|/Game/ThirdPerson/Blueprints/BP_ThirdPersonCharacterCow.BP_ThirdPersonCharacterCow_C|GetMoney _asbp_third_person_character_cow_2) 200)))
              (Rendering|SetActorHiddenInGame true)
              (Collision|SetActorEnableCollision false)
              (bind _asbp_third_person_game_mode (Utilities|Casting|CastToBP_ThirdPersonGameMode (Game|GetGameMode)))
              (Variables|/Game/ThirdPerson/Blueprints/BP_ThirdPersonGameMode.BP_ThirdPersonGameMode_C|SetPuedeSpawnear? _asbp_third_person_game_mode true)
              (Variables|Default|SetDisponible? false)))
          (else
            (Development|PrintString "Ese Delivery no estaba disponible" true true "(R=1.000000,G=0.507329,B=0.000000,A=1.000000)")))))))

(fn ConstructionScript)