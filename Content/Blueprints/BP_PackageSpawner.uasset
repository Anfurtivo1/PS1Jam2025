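; BP_PackageSpawner is a spawner that places BP_Milk package actors at a set of predefined positions.
; Its Spawn function loops through PackagesPositions and, for each not yet in PackagesPositionsOccupied, records it as occupied and spawns a BP_Milk there.
; LiberarPosicion receives each new occupied index but is empty, so positions are never freed here.
; Nothing in this Blueprint calls Spawn.
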(event Collision|EventActorBeginOverlap
  (params (OtherActor :type Actor%20Object%20Reference)))

(fn ConstructionScript)

(fn LiberarPosicion
  (params (Position :type Integer)))

(fn Spawn
  (bind _array_element (Utilities|Array|ForEachLoopwithBreak (Variables|Default|GetPackagesPositions))
    (:LoopBody
      (if (not (Utilities|Array|ContainsItem (Variables|Default|GetPackagesPositionsOccupied) _array_element))
        (bind _returnvalue (Utilities|Array|Add (Variables|Default|GetPackagesPositionsOccupied) _array_element))
        (CallFunction|LiberarPosicion _returnvalue)
        (Game|SpawnActorfromClass "/Game/Blueprints/BP_Milk.BP_Milk_C" (Math|Conversions|ToTransform(Vector) _array_element) "Undefined" "MultiplyWithRoot" 0 0)))))