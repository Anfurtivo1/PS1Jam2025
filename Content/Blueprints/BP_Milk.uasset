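; BP_Milk is a rotating milk package pickup that shows the player's distance in meters on a waypoint widget.
; When the cow character overlaps its box, it increments that character's package count and updates the HUD.
; It then has the game mode free the milk's position, destroys itself and calls PickRandomDelivery.
; The money-decrease timer and Niagara burst logic are unconnected and never run.
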(event OnComponentBeginOverlap(Box)
  (params (OverlappedComponent :type Primitive%20Component%20Object%20Reference) (OtherActor :type Actor%20Object%20Reference) (OtherComp :type Primitive%20Component%20Object%20Reference) (OtherBodyIndex :type Integer) (bFromSweep :type Boolean) (SweepResult :type Hit%20Result%20Structure%20%28by%20ref%29))
  (bind _asbp_third_person_character_cow (Utilities|Casting|CastToBP_ThirdPersonCharacterCow OtherActor))
  (bind _result (Math|Integer|IncrementInt (Variables|/Game/ThirdPerson/Blueprints/BP_ThirdPersonCharacterCow.BP_ThirdPersonCharacterCow_C|GetNumberOfPackages _asbp_third_person_character_cow))
    (:%20%20
      (bind _output_get (Variables|/Game/ThirdPerson/Blueprints/BP_ThirdPersonCharacterCow.BP_ThirdPersonCharacterCow_C|SetNumberOfPackages _asbp_third_person_character_cow _result))
      (Default|SetTxtPackages (Variables|/Game/ThirdPerson/Blueprints/BP_ThirdPersonCharacterCow.BP_ThirdPersonCharacterCow_C|GetHUD _asbp_third_person_character_cow) _output_get)
      (bind _asbp_third_person_game_mode (Utilities|Casting|CastToBP_ThirdPersonGameMode (Game|GetGameMode)))
      (Default|LiberarPosicion _asbp_third_person_game_mode (Variables|/Game/ThirdPerson/Blueprints/BP_ThirdPersonGameMode.BP_ThirdPersonGameMode_C|GetPosicionLeche _asbp_third_person_game_mode))
      (Actor|DestroyActor)
      (Development|PrintString (Utilities|String|Append (Utilities|String|ToString(Integer) (Variables|/Game/ThirdPerson/Blueprints/BP_ThirdPersonGameMode.BP_ThirdPersonGameMode_C|GetPosicionLeche _asbp_third_person_game_mode)) " Es la posicion a eliminar") false true "(R=1.000000,G=0.196227,B=0.245998,A=1.000000)")
      (Default|PickRandomDelivery _asbp_third_person_game_mode))))

(event Custom|MoneyDecrease
  (bind _output_get (Variables|Default|SetMoney (- (Variables|Default|GetMoney) 1e+01)))
  (Development|PrintString (Utilities|String|ToString(Float) (Math|Conversions|ToFloat(Integer) _output_get))))

(event EventBeginPlay
  (Utilities|FlowControl|Sequence
    (:then_0
      (bind _aswd_waypoint (Utilities|Casting|CastToWD_Waypoint (UserInterface|GetWidget (Variables|Default|GetWaypointWidget))))
      (Variables|Default|SetDistance (Variables|/Game/UI/WD_Waypoint.WD_Waypoint_C|GetDistance _aswd_waypoint)))
    (:then_1)))

(event Collision|EventActorBeginOverlap
  (params (OtherActor :type Actor%20Object%20Reference)))

(event EventTick
  (params (DeltaSeconds :type Float%20%28single-precision%29))
  (Transformation|AddLocalRotation (Variables|Default|GetMilk) (Math|Rotator|MakeRotator 0.0 0.0 1.0) false false)
  (Rendering|Components|TextRender|SetText (Variables|Default|GetDistance) (Utilities|Text|ToText(String) (Utilities|String|Append (Utilities|String|ToString(Integer) (Math|Float|Truncate (/ (Math|Vector|Distance(Vector) (Transformation|GetActorLocation) (Transformation|GetActorLocation (Game|Player|GetPlayerPawn 0))) 1e+02))) " m"))))

(fn ConstructionScript)